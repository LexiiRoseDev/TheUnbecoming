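; BP_KeyBook is an interactable book that opens a secret door through a short camera sequence.
; A box overlap toggles input, letting E cut to the book camera and hide the player mesh.
; After delays, a timeline rolls the book, the referenced door opens on its camera, then the mesh reappears with the study camera.
; DoOnce guards only the steps after the initial camera switch and hide.
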(event OnComponentBeginOverlap(Box)
  (params (OverlappedComponent :type Primitive%20Component%20Object%20Reference) (OtherActor :type Actor%20Object%20Reference) (OtherComp :type Primitive%20Component%20Object%20Reference) (OtherBodyIndex :type Integer) (bFromSweep :type Boolean) (SweepResult :type Hit%20Result%20Structure%20%28by%20ref%29))
  (Variables|Default|SetisPlayerInRange true)
  (Input|EnableInput (Game|GetPlayerController 0)))

(event OnComponentEndOverlap(Box)
  (params (OverlappedComponent :type Primitive%20Component%20Object%20Reference) (OtherActor :type Actor%20Object%20Reference) (OtherComp :type Primitive%20Component%20Object%20Reference) (OtherBodyIndex :type Integer))
  (Variables|Default|SetisPlayerInRange false)
  (Input|DisableInput (Game|GetPlayerController 0)))

(event Custom|BookRotation
  (bind _staticmesh (Variables|Default|GetStaticMesh))
  (bind _relativerotation (Variables|/Script/Engine.SceneComponent|GetRelativeRotation _staticmesh))
  (bind _newtrack_0 (Timeline|Rotate%20Book Play)
    (:Update
      (Transformation|SetRelativeRotation _staticmesh (Math|Rotator|MakeRotator _newtrack_0 (.pitch _relativerotation) (.yaw _relativerotation)) false false))))

(event Collision|EventActorBeginOverlap
  (params (OtherActor :type Actor%20Object%20Reference)))

(event EventTick
  (params (DeltaSeconds :type Float%20%28single-precision%29)))

(event Input|KeyboardEvents|E
  (params (Key :type Key%20Structure :default "None"))
  (:Pressed
    (if (Variables|Default|GetisPlayerInRange)
      (Game|Player|SetViewTargetwithBlend (Game|GetPlayerController 0) (Variables|Default|GetBookCam) 0.0 "VTBlend_Linear" 0.0 false)
      (Rendering|SetVisibility (Variables|/Script/Engine.Character|GetMesh (Game|GetPlayerCharacter 0)) false false)
      (Utilities|FlowControl|Delay 1.0)
      (Utilities|FlowControl|DoOnce false
        (:Completed
          (CallFunction|BookRotation)
          (Utilities|FlowControl|Delay 1.2)
          (Game|Player|SetViewTargetwithBlend (Game|GetPlayerController 0) (Variables|Default|GetSecretDoorCam) 0.0 "VTBlend_Linear" 0.0 false)
          (Default|OpenSecretDoor (Variables|Default|GetSecretDoorRef))
          (Utilities|FlowControl|Delay 1.4)
          (Rendering|SetVisibility (Variables|/Script/Engine.Character|GetMesh (Game|GetPlayerCharacter 0)) true false)
          (Game|Player|SetViewTargetwithBlend (Game|GetPlayerController 0) (Variables|Default|GetStudyCam) 0.0 "VTBlend_Linear" 0.0 false))))))

(fn ConstructionScript)