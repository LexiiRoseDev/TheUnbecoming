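; BP_KeyBook is an interactable book that acts as the trigger for opening a secret door.
; Overlapping its box shows an interact widget and enables input, so pressing E in range starts a one-time sequence.
; The sequence hides the player mesh and blends between book and door cameras while a timeline rotates the book and SecretDoorRef opens the door.
; It then restores the mesh, sets StudyCam as the GameMode's current camera, and destroys the box.
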(event OnComponentBeginOverlap(Box)
  (params (OverlappedComponent :type Primitive%20Component%20Object%20Reference) (OtherActor :type Actor%20Object%20Reference) (OtherComp :type Primitive%20Component%20Object%20Reference) (OtherBodyIndex :type Integer) (bFromSweep :type Boolean) (SweepResult :type Hit%20Result%20Structure%20%28by%20ref%29))
  (Variables|Default|SetisPlayerInRange true)
  (Input|EnableInput (Game|GetPlayerController 0))
  (bind _returnvalue (UserInterface|CreateWidget "/Game/Assets/UI/WBP_Interact1.WBP_Interact1_C"))
  (UserInterface|Viewport|AddtoViewport _returnvalue 0))

(event OnComponentEndOverlap(Box)
  (params (OverlappedComponent :type Primitive%20Component%20Object%20Reference) (OtherActor :type Actor%20Object%20Reference) (OtherComp :type Primitive%20Component%20Object%20Reference) (OtherBodyIndex :type Integer))
  (Variables|Default|SetisPlayerInRange false)
  (Input|DisableInput (Game|GetPlayerController 0))
  (Widget|RemovefromParent (stale OnComponentBeginOverlap(Box) _returnvalue)))

(event Custom|BookRotation
  (bind _staticmesh (Variables|Default|GetStaticMesh))
  (bind _relativerotation (Variables|/Script/Engine.SceneComponent|GetRelativeRotation _staticmesh))
  (bind _newtrack_0 (Timeline|Rotate%20Book Play)
    (:Update
      (Transformation|SetRelativeRotation _staticmesh (Math|Rotator|MakeRotator _newtrack_0 (.pitch _relativerotation) (.yaw _relativerotation)) false false))))

(event Input|KeyboardEvents|E
  (params (Key :type Key%20Structure :default "None"))
  (:Pressed
    ;[0.15 0.15 0.15 0.5] Moves the book, moves the door, sets camera angle to study corner.
    (Widget|RemovefromParent (stale OnComponentBeginOverlap(Box) _returnvalue))
    (Utilities|FlowControl|DoOnce false
      (:Completed
        (if (Variables|Default|GetisPlayerInRange)
          (Game|Player|SetViewTargetwithBlend (Game|GetPlayerController 0) (Variables|Default|GetBookCam) 0.0 "VTBlend_Linear" 0.0 false)
          (Rendering|SetVisibility (Variables|/Script/Engine.Character|GetMesh (Game|GetPlayerCharacter 0)) false false)
          (Utilities|FlowControl|Delay 1.0)
          (Utilities|FlowControl|DoOnce false
            (:Completed
              (CallFunction|BookRotation)
              (Utilities|FlowControl|Delay 1.2)
              (Game|Player|SetViewTargetwithBlend (Game|GetPlayerController 0) (Variables|Default|GetSecretDoorCam) 0.0 "VTBlend_Linear" 0.0 false)
              (Default|OpenSecretDoor (Variables|Default|GetSecretDoorRef))
              (Utilities|FlowControl|Delay 1.4)
              (Rendering|SetVisibility (Variables|/Script/Engine.Character|GetMesh (Game|GetPlayerCharacter 0)) true false)
              (bind _asbp_game_mode (Utilities|Casting|CastToBP_GameMode (Game|GetGameMode)))
              (bind _output_get (Variables|/Game/ThirdPerson/Blueprints/BP_GameMode.BP_GameMode_C|SetCurrentCineCam _asbp_game_mode (Variables|Default|GetStudyCam)))
              (Game|Player|SetViewTargetwithBlend (Game|GetPlayerController 0) _output_get 0.0 "VTBlend_Linear" 0.0 false)
              (Components|DestroyComponent (Variables|Default|GetBox)))))))))

(fn ConstructionScript)