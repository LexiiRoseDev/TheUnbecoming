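; BP_Interact is an interactable actor that shows an interaction widget on overlap and a blinking Niagara marker until a letter is read.
; Each Tick it polls IsLetterRead on GI_Main and hides or shows NS_Blink accordingly.
; Begin overlap from any actor sets IsInRange and creates the WBP_Interact widget on screen.
; End overlap clears the flag and removes the widget.
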(event EventTick
  (params (DeltaSeconds :type Float%20%28single-precision%29))
  ;[0.15 0.15 0.15 0.5] Set visibility of NS_Blink component
  (bind _asgi_main (Utilities|Casting|CastToGI_Main (Game|GetGameInstance)))
  (if (Variables|/Game/Assets/GI_Main.GI_Main_C|GetisLetterRead _asgi_main)
    (Rendering|SetVisibility (Variables|Default|GetNS_Blink) false false)
    (else
      (Rendering|SetVisibility (Variables|Default|GetNS_Blink) true false))))

(event Collision|EventActorBeginOverlap
  (params (OtherActor :type Actor%20Object%20Reference))
  (Variables|Default|SetisInRange true)
  (bind _returnvalue (UserInterface|CreateWidget "/Game/Assets/UI/WBP_Interact.WBP_Interact_C"))
  (UserInterface|Viewport|AddtoViewport _returnvalue 0))

(event Collision|EventActorEndOverlap
  (params (OtherActor :type Actor%20Object%20Reference))
  (Variables|Default|SetisInRange false)
  (Widget|RemovefromParent (stale Collision|EventActorBeginOverlap _returnvalue)))

(fn ConstructionScript)