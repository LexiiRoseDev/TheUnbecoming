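; BP_KillBox is a poison zone that drains player health while its trigger volume is overlapped.
; Overlap begin and end toggle IsInRange for any actor, and entry starts a delay loop that repeats a cough sound at the player's location.
; A throttled Tick lowers PlayerHealth in GI_Main while the flag is set, then shows WBP_YouLose when health runs out.
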(event OnComponentBeginOverlap(TriggerVol)
  (params (OverlappedComponent :type Primitive%20Component%20Object%20Reference) (OtherActor :type Actor%20Object%20Reference) (OtherComp :type Primitive%20Component%20Object%20Reference) (OtherBodyIndex :type Integer) (bFromSweep :type Boolean) (SweepResult :type Hit%20Result%20Structure%20%28by%20ref%29))
  ;[0.15 0.15 0.15 0.5] Toggles the boolean for the "poison" event.
  (bind _output_get (Variables|Default|SetisInRange true))
  (Audio|PlaySoundatLocation "/Game/Assets/Sounds/SC_Cough.SC_Cough" (Transformation|GetActorLocation (Game|GetPlayerCharacter 0)) "0, 0, 0" 1.0 1.0 0.0 0 0 0 0 :!label _label)
  (Utilities|FlowControl|Delay 2.0)
  (if _output_get
    (goto _label)))

(event OnComponentEndOverlap(TriggerVol)
  (params (OverlappedComponent :type Primitive%20Component%20Object%20Reference) (OtherActor :type Actor%20Object%20Reference) (OtherComp :type Primitive%20Component%20Object%20Reference) (OtherBodyIndex :type Integer))
  ;[0.15 0.15 0.15 0.5] Toggles the boolean for the "poison" event.
  (Variables|Default|SetisInRange false))

(event EventBeginPlay
  ;[0.15 0.15 0.15 0.5] Set tick speed
  (Actor|Tick|SetActorTickInterval 0.2))

(event EventTick
  (params (DeltaSeconds :type Float%20%28single-precision%29))
  ;[0.15 0.15 0.15 0.5] Checks if player is in range and health > 0, deducts 1% of player health per tick.
  (bind _asgi_main (Utilities|Casting|CastToGI_Main (Game|GetGameInstance)))
  (if (and (> (Variables|/Game/Assets/GI_Main.GI_Main_C|GetPlayerHealth _asgi_main) 0.0) (Variables|Default|GetisInRange))
    (Variables|/Game/Assets/GI_Main.GI_Main_C|SetPlayerHealth _asgi_main (- (Variables|/Game/Assets/GI_Main.GI_Main_C|GetPlayerHealth _asgi_main) 0.01))
    (if (not (> (Variables|/Game/Assets/GI_Main.GI_Main_C|GetPlayerHealth _asgi_main) 0.0))
      (bind _returnvalue (UserInterface|CreateWidget "/Game/Assets/UI/WBP_YouLose.WBP_YouLose_C"))
      (UserInterface|Viewport|AddtoViewport _returnvalue 0))))

(fn ConstructionScript)