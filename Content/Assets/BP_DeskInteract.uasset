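; BP_DeskInteract is an interactable, apparently for a desk, that sends the player to the L_Menu level based on proximity and facing.
; Actor overlap events set an in-range flag and print debug messages.
; Tick opens the level whenever the flag is set and the player character's world yaw is between 0 and 90 degrees, with no key press required.
; The F and N key events only print their key names.
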(event Collision|EventActorBeginOverlap
  (params (OtherActor :type Actor%20Object%20Reference))
  (Variables|Default|SetisInRange true)
  (Development|PrintString "In Range"))

(event Collision|EventActorEndOverlap
  (params (OtherActor :type Actor%20Object%20Reference))
  (Variables|Default|SetisInRange false)
  (Development|PrintString "Not in Range"))

(event EventTick
  (params (DeltaSeconds :type Float%20%28single-precision%29))
  (if (Math|Boolean|ANDBoolean (<= (.Yaw (Math|Rotator|BreakRotator (Transformation|GetActorRotation (Game|GetPlayerCharacter 0)))) 9e+01) (Variables|Default|GetisInRange) (>= (.Yaw (Math|Rotator|BreakRotator (Transformation|GetActorRotation (Game|GetPlayerCharacter 0)))) 0.0))
    (Game|OpenLevel(byName) "L_Menu")))

(event Input|KeyboardEvents|F
  (params (Key :type Key%20Structure :default "None"))
  (:Pressed
    (Development|PrintString "F")))

(event Input|KeyboardEvents|N
  (params (Key :type Key%20Structure :default "None"))
  (:Pressed
    (Development|PrintString "N")))

(fn ConstructionScript)