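; BP_Key is a key pickup actor that is collected by pressing E while in range.
; Its Box overlap events set IsPlayerInRange and toggle input for player controller 0, without checking which actor overlaps.
; Pressing E in range sets IsKeyCollected on the key itself, then immediately destroys the actor.
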(event OnComponentBeginOverlap(Box)
  (params (OverlappedComponent :type Primitive%20Component%20Object%20Reference) (OtherActor :type Actor%20Object%20Reference) (OtherComp :type Primitive%20Component%20Object%20Reference) (OtherBodyIndex :type Integer) (bFromSweep :type Boolean) (SweepResult :type Hit%20Result%20Structure%20%28by%20ref%29))
  (Variables|Default|SetisPlayerInRange true)
  (Input|EnableInput (Game|GetPlayerController 0)))

(event OnComponentEndOverlap(Box)
  (params (OverlappedComponent :type Primitive%20Component%20Object%20Reference) (OtherActor :type Actor%20Object%20Reference) (OtherComp :type Primitive%20Component%20Object%20Reference) (OtherBodyIndex :type Integer))
  (Variables|Default|SetisPlayerInRange false)
  (Input|DisableInput (Game|GetPlayerController 0)))

(event EventBeginPlay)

(event Input|KeyboardEvents|E
  (params (Key :type Key%20Structure :default "None"))
  (:Pressed
    (if (Variables|Default|GetisPlayerInRange)
      (Variables|Default|SetisKeyCollected true)
      (Actor|DestroyActor))))

(fn ConstructionScript)